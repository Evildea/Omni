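; LevelTriggler_BP is a trigger actor that shows a holographic poster while an actor overlaps it, if PosterActive is set.
; BeginPlay hides the poster at zero scale and applies its material.
; Overlap plays the Hologram timeline, reversed on exit, driving poster scale and opacity through the shared PC_Hologram parameter collection.
; An unconnected branch would set hologram saturation from the level's completion state in GuudoGameInstance_BP.
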(event EventBeginPlay
  (|CallParentFunction)
  (bind _output_get (Variables|Default|SetPoster%20Active? (Variables|Default|GetPoster%20Active?)))
  (Transformation|SetWorldScale3D (Variables|Default|GetPoster) "0, 0, 0")
  (Rendering|Material|SetScalarParameterValue "/Game/Assets/PC/PC_Hologram.PC_Hologram" "Opacity Override" 0.0 :!class /Script/Engine.KismetMaterialLibrary)
  (Rendering|Material|SetMaterial (Variables|Default|GetPoster) 0 (Variables|Default|GetPoster%20Material)))

(event Collision|EventActorBeginOverlap
  (params (OtherActor :type Actor%20Object%20Reference))
  (|CallParentFunction OtherActor)
  (if (stale EventBeginPlay _output_get)
    (bind (_direction _x_scale _y_scale _opacity) (Timeline|Hologram PlayFromStart)
      (:Update
        (Transformation|SetWorldScale3D (Variables|Default|GetPoster) (Math|Vector|MakeVector (* _x_scale (Variables|Default|GetPoster%20X%20Scale)) (* _y_scale (Variables|Default|GetPoster%20Y%20Scale)) 2.0))
        (Rendering|Material|SetScalarParameterValue "/Game/Assets/PC/PC_Hologram.PC_Hologram" "Opacity Override" _opacity :!class /Script/Engine.KismetMaterialLibrary)))))

(event Collision|EventActorEndOverlap
  (params (OtherActor :type Actor%20Object%20Reference))
  (|CallParentFunction OtherActor)
  (if (stale EventBeginPlay _output_get)
    (bind (_direction _x_scale _y_scale _opacity) (Timeline|Hologram Reverse)
      (:Update
        (Transformation|SetWorldScale3D (Variables|Default|GetPoster) (Math|Vector|MakeVector (* _x_scale (Variables|Default|GetPoster%20X%20Scale)) (* _y_scale (Variables|Default|GetPoster%20Y%20Scale)) 2.0))
        (Rendering|Material|SetScalarParameterValue "/Game/Assets/PC/PC_Hologram.PC_Hologram" "Opacity Override" _opacity :!class /Script/Engine.KismetMaterialLibrary)))))

(fn ConstructionScript)