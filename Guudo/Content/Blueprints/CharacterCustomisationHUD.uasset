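; CharacterCustomisationHUD sets up the character customisation screen and relays head changes to the character.
; On BeginPlay it caches the first actor implementing BPI_CharacterCustomisation, shows the CharacterCustomiser widget, and switches to UI-only input with a visible cursor.
; Its ChangeHead event forwards the head index to that character through ChangeHeadMessage, with no other customisation handled here.
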(event EventBeginPlay
  (bind _returnvalue (Game|GetPlayerController 0))
  (bind _outactors (Actor|GetAllActorswithInterface "/Game/Blueprints/BPI_CharacterCustomisation.BPI_CharacterCustomisation_C"))
  (Variables|Default|SetCharacter (Utilities|Array|Get(acopy) _outactors))
  (bind _returnvalue_2 (UserInterface|CreateWidget "/Game/HUD/CharacterCustomiser.CharacterCustomiser_C" (Game|GetPlayerController 0)))
  (UserInterface|Viewport|AddtoViewport _returnvalue_2 0)
  (Input|SetInputModeUIOnly _returnvalue _returnvalue_2 "DoNotLock")
  (Variables|/Script/Engine.PlayerController|SetbShowMouseCursor _returnvalue true))

(event Collision|EventActorBeginOverlap
  (params (OtherActor :type Actor%20Object%20Reference)))

(event EventTick
  (params (DeltaSeconds :type Float%20%28single-precision%29)))

(event EventChangeHead
  (params (HeadIndex :type Integer))
  (Class|BPICharacterCustomisation|ChangeHead(Message) (Variables|Default|GetCharacter) HeadIndex))

(fn ConstructionScript)