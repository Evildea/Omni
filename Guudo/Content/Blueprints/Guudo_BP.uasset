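; Guudo_BP is the Guudo character Blueprint, a jelly-bodied character that can grow and shrink between small, normal and large sizes.
; On BeginPlay it applies a physical animation profile below the jelly bone for wobble.
; Each size-change event plays a timeline that feeds UpdateGrowthState and sets the state to Unchanging when finished.
; Tick writes the mesh location to the PC_Outline parameter collection as the player location for materials.
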(event EventBeginPlay
  (bind _jellyphysanim (Variables|Default|GetJellyPhysAnim))
  (Class|PhysicalAnimationComponent|SetSkeletalMeshComponent _jellyphysanim (Variables|Character|GetMesh))
  (Class|PhysicalAnimationComponent|ApplyPhysicalAnimationProfileBelow _jellyphysanim "Jelly_Jnt" "Jelly" false false))

(event EventOnNormaltoLarge
  (bind _size (Timeline|Normal%20to%20Large PlayFromStart)
    (:Update
      (Class|GuudoCharater|UpdateGrowthState _size 1.0))
    (:Finished
      (Class|GuudoCharater|SetGrowthState "Unchanging"))))

(event EventTick
  (params (DeltaSeconds :type Float%20%28single-precision%29))
  (Rendering|Material|SetVectorParameterValue "/Game/Assets/PP/PC_Outline.PC_Outline" "Player Location" (Math|Conversions|ToLinearColor(Vector) (Transformation|GetWorldLocation (Variables|Character|GetMesh))) :!class /Script/Engine.KismetMaterialLibrary))

(event EventOnNormaltoSmall
  (bind _size (Timeline|Normal%20to%20Small PlayFromStart)
    (:Update
      (Class|GuudoCharater|UpdateGrowthState _size 0.0))
    (:Finished
      (Class|GuudoCharater|SetGrowthState "Unchanging"))))

(event EventOnSmalltoNormal
  (bind _size (Timeline|Small%20to%20Normal PlayFromStart)
    (:Update
      (Class|GuudoCharater|UpdateGrowthState _size 0.0))
    (:Finished
      (Class|GuudoCharater|SetGrowthState "Unchanging"))))

(event EventOnLargetoNormal
  (bind _size (Timeline|Large%20to%20Normal PlayFromStart)
    (:Update
      (Class|GuudoCharater|UpdateGrowthState _size 1.0))
    (:Finished
      (Class|GuudoCharater|SetGrowthState "Unchanging"))))

(fn ConstructionScript)