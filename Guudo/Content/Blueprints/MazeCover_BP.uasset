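; MazeCover_BP is a destructible cover piece for a maze that breaks when a Ball touches it.
; On begin play it turns off impulse-on-damage for its Destructible component.
; When a Ball overlaps, it applies damage at the ball's location along its forward vector, then disables the component's collision after a short delay.
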(event EventBeginPlay
  (Variables|/Script/Engine.PrimitiveComponent|SetbApplyImpulseOnDamage (Variables|Default|GetDestructible) false))

(event Collision|EventActorBeginOverlap
  (params (OtherActor :type Actor%20Object%20Reference))
  (bind _asball (Utilities|Casting|CastToBall OtherActor))
  (Utilities|IsValid _asball
    (:Is%20Valid
      (Class|DestructibleComponent|ApplyDamage (Variables|Default|GetDestructible) 1e+02 (Transformation|GetActorLocation OtherActor) (Transformation|GetActorForwardVector OtherActor) 0.0)
      (Utilities|FlowControl|Delay 0.2)
      (Collision|SetCollisionEnabled (Variables|Default|GetDestructible) "NoCollision"))))

(event EventTick
  (params (DeltaSeconds :type Float%20%28single-precision%29)))

(fn ConstructionScript)