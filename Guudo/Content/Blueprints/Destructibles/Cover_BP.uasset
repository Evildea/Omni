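; Destructible cover actor that breaks when hit by either a large Guudo player or a ball, as selected by its DestroyOn setting.
; On static mesh hit, it casts the other actor to the matching type, also requiring Large growth in the player case.
; A valid hit spawns MazeCoverDestroyed_BP at the mesh's world transform, then destroys the intact cover, swapping it for the destroyed version.
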(event OnComponentHit(StaticMesh)
  (params (HitComponent :type Primitive%20Component%20Object%20Reference) (OtherActor :type Actor%20Object%20Reference) (OtherComp :type Primitive%20Component%20Object%20Reference) (NormalImpulse :type Vector :default "0, 0, 0") (Hit :type Hit%20Result%20Structure%20%28by%20ref%29))
  (switch Utilities|FlowControl|Switch|SwitchonDestructionEnumerator (Variables|Designer|GetDestroyOn)
    (:NewEnumerator0
      ;[1 0.9408 0.3957] If Player, make sure they are Large
      (bind _asguudo_bp (Utilities|Casting|CastToGuudo_BP OtherActor))
      (Utilities|IsValid _asguudo_bp
        (:Is%20Valid
          (if (Utilities|Enum|Equal(Enum) (Class|GuudoCharater|GetCurrentGrowth _asguudo_bp) "Large")
            ;[0.3979 1 0.4708] Spawn Destructible
            (Game|SpawnActorfromClass "/Game/Blueprints/Destructibles/Spawns/MazeCoverDestroyed_BP.MazeCoverDestroyed_BP_C" (Transformation|GetWorldTransform (Variables|Default|GetStaticMesh)) "AlwaysSpawn" 0 0 :!label _label)
            (Actor|DestroyActor)))))
    (:NewEnumerator1
      ;[1 0.237 0.4179] If Ball
      (bind _asball (Utilities|Casting|CastToBall OtherActor))
      (Utilities|IsValid _asball
        (:Is%20Valid
          (goto _label))))))

(fn ConstructionScript)