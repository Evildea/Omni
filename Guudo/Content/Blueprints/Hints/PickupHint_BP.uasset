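; PickupHint_BP is a trigger actor that shows a hint popup tied to a pickup target.
; When Guudo_BP overlaps its Box, it creates the Popup widget and adds it to the viewport.
; A flag reset by a timer blocks repeat popups for a cooldown period.
; Tick checks PickupTarget and destroys the hint actor once that target is no longer valid.
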(event OnComponentBeginOverlap(Box)
  (params (OverlappedComponent :type Primitive%20Component%20Object%20Reference) (OtherActor :type Actor%20Object%20Reference) (OtherComp :type Primitive%20Component%20Object%20Reference) (OtherBodyIndex :type Integer) (bFromSweep :type Boolean) (SweepResult :type Hit%20Result%20Structure%20%28by%20ref%29))
  (Utilities|Casting|CastToGuudo_BP OtherActor)
  (if (Variables|Default|GetCanAddToViewport)
    (bind _returnvalue (UserInterface|CreateWidget "/Game/HUD/Popups/Popup.Popup_C"))
    (UserInterface|Viewport|AddtoViewport _returnvalue 0)
    (Variables|Default|SetCanAddToViewport false)
    (Utilities|Time|SetTimerbyEvent (delegate Custom|Reset%20Can%20Add%20To%20Viewport) 1e+01)))

(event Custom|Reset%20Can%20Add%20To%20Viewport
  (Variables|Default|SetCanAddToViewport true))

(event EventTick
  (params (DeltaSeconds :type Float%20%28single-precision%29))
  (Utilities|IsValid (Variables|Designer|GetPickupTarget)
    (:Is%20Not%20Valid
      (Actor|DestroyActor))))

(fn ConstructionScript)